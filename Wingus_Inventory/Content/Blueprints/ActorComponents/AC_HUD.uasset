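; AC_HUD is an actor component that owns the player HUD and toggles it with the Tab key.
; On BeginPlay it creates WBP_PlayerHUD, passing in the owner's AC_Inventory component when one exists.
; Tab adds or removes the widget from the viewport, switching mouse cursor and input mode between Game and UI and game only.
; Each toggle also sends the owner a camera lock message.
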(event `self.ReceiveBeginPlay`
  (bind _output (`|GetArrayItem` (`Actor.K2_GetComponentsByClass` (`self.GetOwner`) "/Game/Blueprints/ActorComponents/AC_Inventory.AC_Inventory_C")))
  (`/Engine/EditorBlueprintResources/StandardMacros.IsValid` _output
    (:`Is Valid`
      (bind _returnvalue (`|CreateWidget` "/Game/UI/WBP_PlayerHUD.WBP_PlayerHUD_C" (`GameplayStatics.GetPlayerController` 0) _output))
      (set `self.HUD Widget` _returnvalue))))

(event `Key|Tab`
  (params (Key :type "Key Structure"))
  (bind _returnvalue (`self.GetOwner`))
  (bind _returnvalue_2 (`PlayerState.GetPlayerController` (`GameplayStatics.GetPlayerState` 0)))
  (:`Pressed`
    (if (`Widget.IsVisible` (`self.HUD Widget`))
      (`Widget.RemoveFromParent` (`self.HUD Widget`))
      (set `PlayerController.bShowMouseCursor` false (`PlayerState.GetPlayerController` (`GameplayStatics.GetPlayerState` 0)))
      (message `/Game/Blueprints/Interfaces/BPI_Player.SetCameraLock` _returnvalue false)
      (`WidgetBlueprintLibrary.SetInputMode_GameOnly` _returnvalue_2)
      (else
        (`UserWidget.AddToViewport` (`self.HUD Widget`) 0)
        (set `PlayerController.bShowMouseCursor` true (`PlayerState.GetPlayerController` (`GameplayStatics.GetPlayerState` 0)))
        (message `/Game/Blueprints/Interfaces/BPI_Player.SetCameraLock` _returnvalue true)
        (`WidgetBlueprintLibrary.SetInputMode_GameAndUIEx` _returnvalue_2 (`self.HUD Widget`) "DoNotLock" false)))))