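; Actor component that gives its owner a 20-slot inventory of item ID and amount pairs, with a Tab-toggled UI panel.
; Functions add, find and remove items, stack or swap slots within or between inventories, and drop items as impulse-launched pickups.
; Most changes fire an update notification; the panel receives the component on creation.
; Toggling the panel switches cursor, input mode and camera lock, and a debug Q key removes a "White Ball".
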(event Custom|Event%20Inventory%20Updated
  (Default|CallOnInventoryUpdated))

(event EventBeginPlay
  (bind _returnvalue (UserInterface|CreateWidget "/Game/UI/Inventory/WBP_Inventory.WBP_Inventory_C" 0 self))
  (Utilities|Array|Resize (Variables|Default|GetItems) 20)
  (Variables|Default|SetInventory%20Panel _returnvalue))

(event Input|KeyboardEvents|DebugKeyQ
  (params (Key :type Key%20Structure) (ActionValue :type Input%20Action%20Value%20Structure))
  (:Pressed
    (bind _amount_removed (CallFunction|RemoveItem (Utilities|String|StringToName (Utilities|String|MakeLiteralString "White Ball")) 1 true))
    (Development|PrintString (Utilities|String|Append "Removed " (Utilities|String|ToString(Integer) _amount_removed) " White Ball(s)"))))

(event Input|KeyboardEvents|Tab
  (params (Key :type Key%20Structure))
  (bind _returnvalue (Game|GetPlayerState 0))
  (bind _returnvalue_2 (Components|GetOwner))
  (bind _inventory_panel (Variables|Default|GetInventory%20Panel))
  (bind _returnvalue_3 (Game|GetPlayerController _returnvalue))
  (:Pressed
    (if (Widget|IsVisible (Variables|Default|GetInventory%20Panel))
      (Widget|RemovefromParent _inventory_panel)
      (Variables|/Script/Engine.PlayerController|SetbShowMouseCursor (Game|GetPlayerController (Game|GetPlayerState 0)) false)
      (Class|BPIPlayer|SetCameraLock(Message) _returnvalue_2 false)
      (Input|SetInputModeGameOnly _returnvalue_3 false)
      (else
        (UserInterface|Viewport|AddtoViewport _inventory_panel 0)
        (Variables|/Script/Engine.PlayerController|SetbShowMouseCursor (Game|GetPlayerController (Game|GetPlayerState 0)) true)
        (Class|BPIPlayer|SetCameraLock(Message) _returnvalue_2 true)
        (Input|SetInputModeGameandUI _returnvalue_3 (Variables|Default|GetInventory%20Panel) "DoNotLock" false false)))))

(fn AddItem
  (params (Item%20ID :type Name) (Amount :type Integer))
  ;[0.15 0.15 0.15 0.5] Check if we already have this
  (bind (_array_element _array_index) (Utilities|Array|ForEachLoopwithBreak (Variables|Default|GetItems) :!label _label)
    (:LoopBody
      (if (== Item%20ID (.ID (Utilities|Struct|BreakF_InventorySlot _array_element)))
        (LocalVariables|SetItem%20Already%20Exists true)
        (Utilities|Struct|SetmembersinF_InventorySlot (Utilities|Array|Get(acopy) (Variables|Default|GetItems) _array_index) (+ (.Amount (Utilities|Struct|BreakF_InventorySlot _array_element)) Amount))
        (Default|CallOnInventoryUpdated)
        (goto _label Break)))
    (:Completed
      ;[0.15 0.15 0.15 0.5] If we don't have this, add it
      (if (LocalVariables|GetItem%20Already%20Exists)
        (return true 0)
        (else
          (bind (_array_element_2 _array_index_2) (Utilities|Array|ForEachLoopwithBreak (Variables|Default|GetItems))
            (:LoopBody
              (if (== (.id _array_element_2) "")
                (Utilities|Array|SetArrayElem (Variables|Default|GetItems) _array_index_2 (Utilities|Struct|MakeF_InventorySlot Item%20ID Amount))
                (Default|CallOnInventoryUpdated)
                (return true Amount)))
            (:Completed
              (Default|CallOnInventoryUpdated)
              (return false 0))))))))

(fn AddbyIndex
  (params (Item%20ID :type Name) (Amount :type Integer) (Index :type Integer))
  (bind _items (Variables|Default|GetItems))
  (bind _returnvalue (Utilities|Array|LastIndex _items))
  (bind _index (Utilities|FlowControl|ForLoopwithBreak 0 _returnvalue)
    (:LoopBody
      (if (== (.ID (Utilities|Struct|BreakF_InventorySlot (Utilities|Array|Get(acopy) (Variables|Default|GetItems) (Class|KismetMathLibrary|Wrap (+ _index Index) -1 _returnvalue)))) "")
        (Utilities|Array|SetArrayElem (Variables|Default|GetItems) (Class|KismetMathLibrary|Wrap (+ _index Index) -1 _returnvalue) (Utilities|Struct|MakeF_InventorySlot Item%20ID Amount))
        (return true Amount (Class|KismetMathLibrary|Wrap (+ _index Index) -1 _returnvalue))))
    (:Completed
      (return false 0 -1))))

(fn RemoveItem
  (params (ID :type Name) (Amount :type Integer) (Allow%20Partial :type Boolean))
  (bind (_found_item _indices) (CallFunction|FindItem ID))
  (if _found_item
    (LocalVariables|SetTarget%20Index (Utilities|Array|Get(acopy) _indices))
    (if (> (.Amount (Utilities|Struct|BreakF_InventorySlot (Utilities|Array|Get(acopy) (Variables|Default|GetItems) (LocalVariables|GetTarget%20Index)))) 0)
      (Utilities|Struct|SetmembersinF_InventorySlot (Utilities|Array|Get(acopy) (Variables|Default|GetItems) (LocalVariables|GetTarget%20Index)) (- (.Amount (Utilities|Struct|BreakF_InventorySlot (Utilities|Array|Get(acopy) (Variables|Default|GetItems) (LocalVariables|GetTarget%20Index)))) Amount))
      (Default|CallOnInventoryUpdated)
      (return Amount)
      (elif (or Allow%20Partial (== (.Amount (Utilities|Struct|BreakF_InventorySlot (Utilities|Array|Get(acopy) (Variables|Default|GetItems) (LocalVariables|GetTarget%20Index)))) Amount))
        (LocalVariables|SetTemp (.Amount (Utilities|Struct|BreakF_InventorySlot (Utilities|Array|Get(acopy) (Variables|Default|GetItems) (LocalVariables|GetTarget%20Index)))))
        (Utilities|Struct|SetmembersinF_InventorySlot (Utilities|Array|Get(acopy) (Variables|Default|GetItems) (LocalVariables|GetTarget%20Index)) "None")
        (Default|CallOnInventoryUpdated)
        (return (LocalVariables|GetTemp))
        (else
          (return 0))))
    (else
      (return 0))))

(fn RemovebyIndex
  (params (Index :type Integer) (Amount :type Integer) (Allow%20Partial :type Boolean))
  (bind _items (Variables|Default|GetItems))
  (bind _output (Utilities|Array|Get(acopy) _items Index))
  (if (> (.Amount (Utilities|Struct|BreakF_InventorySlot (Utilities|Array|Get(acopy) (Variables|Default|GetItems) Index))) Amount)
    (Utilities|Struct|SetmembersinF_InventorySlot _output (- (.Amount (Utilities|Struct|BreakF_InventorySlot _output)) Amount))
    (Default|CallOnInventoryUpdated)
    (return Amount)
    (elif (or Allow%20Partial (== (.Amount (Utilities|Struct|BreakF_InventorySlot (Utilities|Array|Get(acopy) (Variables|Default|GetItems) Index))) Amount))
      (LocalVariables|SetPartial%20Amount (.Amount (Utilities|Struct|BreakF_InventorySlot (Utilities|Array|Get(acopy) (Variables|Default|GetItems) Index))))
      (Utilities|Struct|SetmembersinF_InventorySlot (Utilities|Array|Get(acopy) (Variables|Default|GetItems) Index) "None")
      (Default|CallOnInventoryUpdated)
      (return (LocalVariables|GetPartial%20Amount))
      (else
        (return 0)))))

(fn FindItem
  (params (Item%20ID :type Name))
  (bind _target_indices (LocalVariables|GetTarget%20Indices))
  (bind (_array_element _array_index) (Utilities|Array|ForEachLoopwithBreak (Variables|Default|GetItems))
    (:LoopBody
      (if (== Item%20ID (.ID (Utilities|Struct|BreakF_InventorySlot _array_element)))
        (Utilities|Array|Add (LocalVariables|GetTarget%20Indices) _array_index)))
    (:Completed
      (return (Utilities|Array|IsNotEmpty _target_indices) _target_indices))))

(fn TransferItems
  (params (Source%20Index :type Integer) (Destination%20Index :type Integer) (Source%20Inventory :type AC%20Inventory%20Object%20Reference))
  (bind _items (Variables|Default|GetItems))
  (bind _output (Utilities|Array|Get(acopy) _items Destination%20Index))
  (LocalVariables|SetSource%20Item (Utilities|Array|Get(acopy) (Variables|AC_Inventory_C|GetItems Source%20Inventory) Source%20Index))
  (if (not (< Destination%20Index 0))
    (if (== (.ID (Utilities|Struct|BreakF_InventorySlot (LocalVariables|GetSource%20Item))) (.ID (Utilities|Struct|BreakF_InventorySlot (Utilities|Array|Get(acopy) (Variables|Default|GetItems) Destination%20Index))))
      ;[0.15 0.15 0.15 0.5] Items are same
      (Utilities|Struct|SetmembersinF_InventorySlot _output (+ (.Amount (Utilities|Struct|BreakF_InventorySlot (LocalVariables|GetSource%20Item))) (.Amount (Utilities|Struct|BreakF_InventorySlot _output))))
      (CallFunction|RemovebyIndex Source%20Inventory Source%20Index (.Amount (Utilities|Struct|BreakF_InventorySlot (LocalVariables|GetSource%20Item))) false)
      (CallFunction|EventInventoryUpdated)
      (if (!= Source%20Inventory self)
        (CallFunction|EventInventoryUpdated Source%20Inventory))
      (else
        ;[0.15 0.15 0.15 0.5] Items are different
        (Utilities|Array|SetArrayElem (Variables|AC_Inventory_C|GetItems Source%20Inventory) Source%20Index (Utilities|Array|Get(acopy) (Variables|Default|GetItems) Destination%20Index))
        (Utilities|Array|SetArrayElem (Variables|Default|GetItems) Destination%20Index (LocalVariables|GetSource%20Item))
        (CallFunction|EventInventoryUpdated)
        (if (!= Source%20Inventory self)
          (CallFunction|EventInventoryUpdated Source%20Inventory))))))

(fn SpawnItem
  (params (Item%20ID :type Name) (Amount :type Integer))
  (bind _returnvalue (Components|GetOwner))
  (bind _returnvalue_2 (Math|Random|RandomUnitVector))
  (bind _returnvalue_3 (Math|Float|MakeLiteralFloat 5e+01))
  (bind _returnvalue_4 (Transformation|GetActorLocation _returnvalue))
  (bind _returnvalue_5 (Transformation|GetActorForwardVector _returnvalue))
  (bind _returnvalue_6 (* _returnvalue_2 _returnvalue_3))
  (bind _returnvalue_7 (* _returnvalue_5 2.5e+02))
  (bind _returnvalue_8 (+ _returnvalue_6 _returnvalue_7))
  (bind _aspawn (Utilities|Casting|CastToPawn _returnvalue)
    (:then
      (bind _returnvalue_9 (Game|SpawnActorfromClass "/Game/Blueprints/BP_ItemPickup.BP_ItemPickup_C" (Math|Transform|MakeTransform _returnvalue_4 "0, 0, 0" "1.000000,1.000000,1.000000") "Undefined" "MultiplyWithRoot" 0 Item%20ID Amount _aspawn))
      (Physics|AddImpulse (Variables|/Game/Blueprints/BP_ItemPickup.BP_ItemPickup_C|GetCube _returnvalue_9) _returnvalue_8 "None" true))
    (:CastFailed
      (bind _returnvalue_10 (Game|SpawnActorfromClass "/Game/Blueprints/BP_ItemPickup.BP_ItemPickup_C" (Math|Transform|MakeTransform _returnvalue_4 "0, 0, 0" "1.000000,1.000000,1.000000") "Undefined" "MultiplyWithRoot" 0 Item%20ID Amount 0))
      (Physics|AddImpulse (Variables|/Game/Blueprints/BP_ItemPickup.BP_ItemPickup_C|GetCube _returnvalue_10) _returnvalue_8 "None" true))))