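; Actor component that lets its owning Character select and interact with nearby actors implementing BPI_Interact.
; Capsule overlap events maintain an in-range list, selecting the latest arrival and clamping the index on exit.
; The mouse wheel cycles the selection with wraparound, sending preview enter/exit messages as it changes.
; Pressing E sends InteractMessage to the selected actor with the owner as argument.
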(event `self.ReceiveBeginPlay`
  (bind _ascharacter (cast `Character` (`self.GetOwner`)))
  (bind _capsulecomponent (`Character.CapsuleComponent` _ascharacter))
  (add `PrimitiveComponent.OnComponentBeginOverlap` _capsulecomponent (`|CreateDelegate` :!event `Component Begin Overlap`))
  (add `PrimitiveComponent.OnComponentEndOverlap` _capsulecomponent (`|CreateDelegate` :!event `Component End Overlap`)))

(event `Component Begin Overlap`
  (params (OverlappedComponent :type "PrimitiveComponent Object Reference") (OtherActor :type "Actor Object Reference") (OtherComp :type "PrimitiveComponent Object Reference") (OtherBodyIndex :type Integer) (bFromSweep :type Boolean) (SweepResult :type "HitResult Structure (by ref)"))
  (if (`KismetSystemLibrary.DoesImplementInterface` OtherActor "/Game/Blueprints/Interfaces/BPI_Interact.BPI_Interact_C")
    (bind _returnvalue (`KismetArrayLibrary.Array_AddUnique` (`self.Interactables In Range`) OtherActor))
    (set `self.SelectedInteractableIndex` _returnvalue)
    (`self.UpdateSelectedInteractable`)))

(event `Component End Overlap`
  (params (OverlappedComponent :type "PrimitiveComponent Object Reference") (OtherActor :type "Actor Object Reference") (OtherComp :type "PrimitiveComponent Object Reference") (OtherBodyIndex :type Integer))
  (if (`KismetSystemLibrary.DoesImplementInterface` OtherActor "/Game/Blueprints/Interfaces/BPI_Interact.BPI_Interact_C")
    (`KismetArrayLibrary.Array_RemoveItem` (`self.Interactables In Range`) OtherActor)
    (`self.ClampIndexInBounds`)
    (`self.UpdateSelectedInteractable`)))

(event `Key|E`
  (params (Key :type "Key Structure"))
  (:`Pressed`
    (message `/Game/Blueprints/Interfaces/BPI_Interact.Interact` (`self.SelectedInteractable`) (`self.GetOwner`))
    (`self.ClampIndexInBounds`)))

(event `InputAxisKey|MouseWheelAxis`
  (params (AxisValue :type "Float (single-precision)"))
  (bind _returnvalue (+ (`KismetMathLibrary.SignOfInteger` (`KismetMathLibrary.FTrunc` AxisValue)) (`self.SelectedInteractableIndex`)))
  (if (!= 0.0 AxisValue)
    (if (> _returnvalue (`KismetArrayLibrary.Array_LastIndex` (`self.Interactables In Range`)))
      (set `self.SelectedInteractableIndex` 0)
      (`self.UpdateSelectedInteractable`)
      (elif (< _returnvalue 0)
        (set `self.SelectedInteractableIndex` (`KismetArrayLibrary.Array_LastIndex` (`self.Interactables In Range`)))
        (`self.UpdateSelectedInteractable`)
        (else
          (set `self.SelectedInteractableIndex` _returnvalue)
          (`self.UpdateSelectedInteractable`))))))

(fn `ClampIndexInBounds`
  (set `self.SelectedInteractableIndex` (`KismetMathLibrary.Clamp` (`self.SelectedInteractableIndex`) 0 (`KismetArrayLibrary.Array_LastIndex` (`self.Interactables In Range`)))))

(fn `UpdateSelectedInteractable`
  (bind _selectedinteractable (`self.SelectedInteractable`))
  (if (!= (`|GetArrayItem` (`self.Interactables In Range`) (`self.SelectedInteractableIndex`)) (`self.SelectedInteractable`))
    (`|ExecutionSequence`
      (:`then_0`
        (if (`KismetSystemLibrary.IsValid` _selectedinteractable)
          (message `/Game/Blueprints/Interfaces/BPI_Interact.Interact Preview Exit` _selectedinteractable)))
      (:`then_1`
        (bind _output_get (set `self.SelectedInteractable` (`|GetArrayItem` (`self.Interactables In Range`) (`self.SelectedInteractableIndex`))))
        (message `/Game/Blueprints/Interfaces/BPI_Interact.Interact Preview Enter` _output_get)))))