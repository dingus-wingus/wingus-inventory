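; BP_ItemPickup is a world item that an interacting actor can pick up into its inventory.
; On BeginPlay it feeds its ItemID and Amount to a hidden WBP_PickUpPreview widget, which the interact preview enter and exit events show and hide.
; Interact calls AddItem on the interactor's AC_Inventory component and destroys the pickup only if the item was added.
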(event `self.ReceiveBeginPlay`
  (bind _returnvalue (`WidgetComponent.GetWidget` (`self.Widget`)))
  (`Widget.SetVisibility` _returnvalue "Collapsed")
  (bind _aswbp_pick_up_preview (cast `/Game/UI/Interaction/WBP_PickUpPreview` _returnvalue))
  (`/Game/UI/Interaction/WBP_PickUpPreview.LoadItem` _aswbp_pick_up_preview (make `/Game/Data/F_InventorySlot` (`self.Item ID`) (`self.Amount`))))

(event `/Game/Blueprints/Interfaces/BPI_Interact.Interact`
  (params (Interactor :type "Actor Object Reference"))
  (bind _output (`|GetArrayItem` (`self.K2_GetComponentsByClass` Interactor "/Game/Blueprints/ActorComponents/AC_Inventory.AC_Inventory_C")))
  (`/Engine/EditorBlueprintResources/StandardMacros.IsValid` _output
    (:`Is Valid`
      (bind _item_added (`/Game/Blueprints/ActorComponents/AC_Inventory.AddItem` _output (`self.Item ID`) (`self.Amount`)))
      (if _item_added
        (`self.K2_DestroyActor`)))))

(event `/Game/Blueprints/Interfaces/BPI_Interact.Interact Preview Enter`
  (`Widget.SetVisibility` (`WidgetComponent.GetWidget` (`self.Widget`)) "HitTestInvisible"))

(event `/Game/Blueprints/Interfaces/BPI_Interact.Interact Preview Exit`
  (bind _returnvalue (`WidgetComponent.GetWidget` (`self.Widget`)))
  (`/Engine/EditorBlueprintResources/StandardMacros.IsValid` _returnvalue
    (:`Is Valid`
      (`Widget.SetVisibility` _returnvalue "Collapsed"))))

(fn `UserConstructionScript`)