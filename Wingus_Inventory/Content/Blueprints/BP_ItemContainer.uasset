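; BP_ItemContainer is an interactable container actor that opens an inventory menu between itself and whoever interacts with it.
; On BeginPlay it hides its prompt widget and pre-creates a WBP_ContainerMenu bound to its own AC_Inventory.
; Interact feeds the interactor's AC_Inventory into that menu, shows it, then enables the cursor, UI-only input and a camera lock.
; Preview enter and exit events toggle the interaction prompt's visibility.
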(event `self.ReceiveBeginPlay`
  (`Widget.SetVisibility` (`WidgetComponent.GetWidget` (`self.Interact Widget`)) "Collapsed")
  (bind _returnvalue (`|CreateWidget` "/Game/UI/Inventory/WBP_ContainerMenu.WBP_ContainerMenu_C" (`GameplayStatics.GetPlayerController` 0) (`self.AC_Inventory`)))
  (set `self.Container Menu` _returnvalue))

(event `/Game/Blueprints/Interfaces/BPI_Interact.Interact`
  (params (Interactor :type "Actor Object Reference"))
  (bind _returnvalue (`GameplayStatics.GetPlayerController` 0))
  (bind _output (`|GetArrayItem` (`self.K2_GetComponentsByClass` Interactor "/Game/Blueprints/ActorComponents/AC_Inventory.AC_Inventory_C")))
  (bind _interactorinventory (`/Game/UI/Inventory/WBP_ContainerMenu.InteractorInventory` (`self.Container Menu`)))
  (`/Engine/EditorBlueprintResources/StandardMacros.IsValid` _output
    (:`Is Valid`
      (set `self.Interactor Inventory Comp` _output)
      (`UserWidget.AddToViewport` (`self.Container Menu`) 0)
      (set `PlayerController.bShowMouseCursor` true (`GameplayStatics.GetPlayerController` 0))
      (message `/Game/Blueprints/Interfaces/BPI_Player.SetCameraLock` _returnvalue true)
      (`WidgetBlueprintLibrary.SetInputMode_UIOnlyEx` _returnvalue (`self.Container Menu`))
      (`UserWidget.SetOwningPlayer` (`self.Container Menu`) (`GameplayStatics.GetPlayerController` 0))
      (set `/Game/UI/Inventory/WBP_Inventory.Inventory Component` (`self.Interactor Inventory Comp`) _interactorinventory)
      (`/Game/UI/Inventory/WBP_Inventory.Initialize` _interactorinventory))))

(event `/Game/Blueprints/Interfaces/BPI_Interact.Interact Preview Enter`
  (`Widget.SetVisibility` (`WidgetComponent.GetWidget` (`self.Interact Widget`)) "HitTestInvisible"))

(event `/Game/Blueprints/Interfaces/BPI_Interact.Interact Preview Exit`
  (bind _returnvalue (`WidgetComponent.GetWidget` (`self.Interact Widget`)))
  (`/Engine/EditorBlueprintResources/StandardMacros.IsValid` _returnvalue
    (:`Is Valid`
      (`Widget.SetVisibility` _returnvalue "Collapsed"))))

(fn `UserConstructionScript`)